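; Cube physics object in the GravityVectorGun feature's set of physics objects.
; Its construction script runs the parent's script, then gives PhysicsMesh the Cube static mesh and a first-person colorway material, and turns on physics simulation.
; The event graph holds only disabled default events, so this Blueprint adds no runtime logic of its own.
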(fn `UserConstructionScript`
  (bind _physicsmesh (`self.PhysicsMesh`))
  (`parent.UserConstructionScript`)
  (`StaticMeshComponent.SetStaticMesh` _physicsmesh "/Engine/BasicShapes/Cube.Cube")
  (`PrimitiveComponent.SetMaterial` _physicsmesh 0 "/Game/FirstPerson/MI_FirstPersonColorway.MI_FirstPersonColorway")
  (`PrimitiveComponent.SetSimulatePhysics` (`self.PhysicsMesh`) true))