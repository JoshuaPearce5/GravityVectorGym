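; BP_Goal is a goal trigger in the gravity vector gun game that reacts when a specific physics object reaches it.
; When its box overlaps the assigned RequiredObject, it casts DoorToOpen to BP_PhysicsObject_Base and enables its custom gravity, so the door is itself a physics object.
; It also swaps the cube to a green material and plays a success sound as feedback.
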(event `self.ReceiveBeginPlay`)

(event `self.Box.OnComponentBeginOverlap`
  (params (OverlappedComponent :type "PrimitiveComponent Object Reference") (OtherActor :type "Actor Object Reference") (OtherComp :type "PrimitiveComponent Object Reference") (OtherBodyIndex :type Integer) (bFromSweep :type Boolean) (SweepResult :type "HitResult Structure (by ref)"))
  (bind _asbp_physics_object_base (cast `/Game/GravityVectorGun/PhysicsObjects/BP_PhysicsObject_Base` OtherActor))
  (if (== _asbp_physics_object_base (`self.RequiredObject`))
    (bind _asbp_physics_object_base_2 (cast `/Game/GravityVectorGun/PhysicsObjects/BP_PhysicsObject_Base` (`self.DoorToOpen`)))
    (set `/Game/GravityVectorGun/PhysicsObjects/BP_PhysicsObject_Base.CustomGravityEnabled` true _asbp_physics_object_base_2)
    (`PrimitiveComponent.SetMaterial` (`self.Cube`) 0 "/AnimationSharing/AnimSharingGreen.AnimSharingGreen")
    (`GameplayStatics.PlaySound2D` "/Game/GravityVectorGun/SW_Success.SW_Success" 1.0 1.0 0.0 null (`GameplayStatics.GetPlayerPawn` 0))))

(fn `UserConstructionScript`)